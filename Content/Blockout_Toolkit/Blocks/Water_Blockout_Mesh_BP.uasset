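; Blockout water block that displays a resizable plane with a tintable water material for level prototyping.
; The construction script creates a dynamic instance of Water_M, assigns it to the plane, then refreshes colors and size.
; RefreshMaterial pushes the color, depth color and foam color properties into the material, and UpdateSize scales the plane from Size divided by 100.
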(fn ConstructionScript
  (bind _returnvalue (Rendering|Material|CreateDynamicMaterialInstance "/Game/Blockout_Toolkit/Materials/Water_M.Water_M" "None" "None" :!class /Script/Engine.KismetMaterialLibrary))
  (bind _output_get (Variables|Runtime|SetMaterial%20Instance _returnvalue))
  (Rendering|Material|SetMaterial (Variables|Default|GetPlane) 0 _output_get)
  (CallFunction|RefreshMaterial)
  (CallFunction|UpdateSize))

(fn UpdateSize
  (Transformation|SetRelativeScale3D (Variables|Default|GetPlane) (/ (Variables|Settings|GetSize) 100)))

(fn RefreshMaterial
  (Rendering|Material|SetVectorParameterValue (Variables|Runtime|GetMaterial%20Instance) "Color" (Variables|Settings|GetColor) :!class /Script/Engine.MaterialInstanceDynamic)
  (Rendering|Material|SetVectorParameterValue (Variables|Runtime|GetMaterial%20Instance) "Depth Color" (Variables|Settings|GetDepth%20Color) :!class /Script/Engine.MaterialInstanceDynamic)
  (Rendering|Material|SetVectorParameterValue (Variables|Runtime|GetMaterial%20Instance) "Foam Color" (Variables|Settings|GetFoam%20Color) :!class /Script/Engine.MaterialInstanceDynamic))