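; BP_ExitGate is an interactable exit gate that stays inactive until the CipherManager's gate-active dispatcher fires.
; On begin play it hides its spotlight and both prompts and binds to that dispatcher, which later lights the spotlight, shows the activated prompt and sets GateActivated.
; Interacting with an activated gate swaps to the decoded prompt and plays a Timeline that slides the two doors by relative location.
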(event Custom|ActivateGate
  ;[1 1 1] Gate Activation
  (Rendering|SetVisibility (Variables|Default|GetSpotLight) true false)
  (Variables|Default|SetGateActivated true)
  (Rendering|SetVisibility (Variables|Default|GetPromptActivated) true false))

(event EventBeginPlay
  ;[1 1 1] Gate Activation
  (Rendering|SetVisibility (Variables|Default|GetSpotLight) false false)
  (Rendering|SetVisibility (Variables|Default|GetPromptDecoded) false false)
  (Rendering|SetVisibility (Variables|Default|GetPromptActivated) false false)
  (EventDispatchers|BindEventtoGateActiveDispatcher (Variables|Default|GetCipherManager) (delegate Custom|ActivateGate)))

(event Collision|EventActorBeginOverlap
  (params (OtherActor :type Actor%20Object%20Reference)))

(event EventTick
  (params (DeltaSeconds :type Float%20%28single-precision%29))
  (|CallParentFunction DeltaSeconds) ; This node is disabled and will not be called.\nDrag off pins to build functionality.
)

(event EventInteract
  ;[1 1 1] Gate Opening
  (if (Variables|Default|GetGateActivated)
    (Rendering|SetVisibility (Variables|Default|GetPromptDecoded) true false)
    (Rendering|SetVisibility (Variables|Default|GetPromptActivated) false false)
    (bind (_direction _door1_xvector _door2_xvector) (Timeline|Timeline Play)
      (:Update
        (Transformation|SetRelativeLocation (Variables|Default|GetDoor1) _door1_xvector false false)
        (Transformation|SetRelativeLocation (Variables|Default|GetDoor2) _door2_xvector false false)))))

(fn ConstructionScript
  (|CallParentFunction))