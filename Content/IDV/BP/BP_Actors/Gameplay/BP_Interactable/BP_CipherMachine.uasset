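; BP_CipherMachine is an interactable cipher machine actor that can be decoded once.
; Its spotlight and prompt components start hidden on BeginPlay.
; Interact, if the machine is still interactable, reveals both components, clears the Interactable flag and calls the cipher dispatcher to signal the decode.
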(event EventBeginPlay
  (Rendering|SetVisibility (Variables|Default|GetSpotLight) false false)
  (Rendering|SetVisibility (Variables|Default|GetPrompt) false false))

(event Collision|EventActorBeginOverlap
  (params (OtherActor :type Actor%20Object%20Reference)))

(event EventTick
  (params (DeltaSeconds :type Float%20%28single-precision%29)))

(event EventInteract
  ;[1 1 1] Cipher Decoded
  (if (Variables|Default|GetInteractable)
    (Rendering|SetVisibility (Variables|Default|GetSpotLight) true false)
    (Rendering|SetVisibility (Variables|Default|GetPrompt) true false)
    (Variables|Default|SetInteractable false)
    (Default|CallCipherDispatcher)))

(fn ConstructionScript)