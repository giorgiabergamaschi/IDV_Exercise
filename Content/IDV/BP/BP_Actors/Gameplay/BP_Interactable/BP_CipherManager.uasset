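; Cipher manager actor that tracks cipher completion and signals when the dungeon and gate become active.
; On BeginPlay it binds its CipherCheck event to the dispatcher of every cipher in its Ciphers array.
; Each cipher callback increments a completion counter, firing the dungeon-active dispatcher at two completions and the gate-active dispatcher at five.
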(event Custom|CipherCheck
  ;[1 1 1] Cipher Check
  (bind _result (Math|Integer|IncrementInt (Variables|Default|GetCipherCompletion))
    (:%20%20
      (if (== _result 5)
        (Default|CallGateActiveDispatcher)
        (elif (== _result 2)
          (Default|CallDungeonActiveDispatcher))))))

(event EventBeginPlay
  ;[1 1 1] Cipher Check
  (for _array_element (Variables|Default|GetCiphers)
    (EventDispatchers|BindEventtoCipherDispatcher _array_element (delegate Custom|CipherCheck))))

(event Collision|EventActorBeginOverlap
  (params (OtherActor :type Actor%20Object%20Reference)))

(event EventTick
  (params (DeltaSeconds :type Float%20%28single-precision%29)))

(fn ConstructionScript)